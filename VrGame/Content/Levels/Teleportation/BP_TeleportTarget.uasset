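; BP_TeleportTarget is a projectile actor that teleports the player to where it hits.
; When its Sphere component registers a hit, it moves player pawn 0 to its own location, keeping the pawn's rotation, then destroys itself.
; BeginPlay, projectile bounce and stop, and the hit itself print debug strings.
; An alternative teleport branch with a debug draw is left disconnected and never runs.
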(event `self.ReceiveBeginPlay`
  (`KismetSystemLibrary.PrintString` "spawned"))

(event `self.ProjectileMovement.OnProjectileBounce`
  (params (ImpactResult :type "HitResult Structure (by ref)") (ImpactVelocity :type "Vector Structure (by ref)"))
  (`KismetSystemLibrary.PrintString` "Hello" :!label _label))

(event `self.ProjectileMovement.OnProjectileStop`
  (params (ImpactResult :type "HitResult Structure (by ref)"))
  (goto _label))

(event `self.Sphere.OnComponentHit`
  (params (HitComponent :type "PrimitiveComponent Object Reference") (OtherActor :type "Actor Object Reference") (OtherComp :type "PrimitiveComponent Object Reference") (NormalImpulse :type "Vector Structure") (Hit :type "HitResult Structure (by ref)"))
  (bind _returnvalue (`GameplayStatics.GetPlayerPawn` 0))
  (`KismetSystemLibrary.PrintString` (`KismetStringLibrary.Conv_ObjectToString` OtherActor))
  (`self.K2_TeleportTo` _returnvalue (`self.K2_GetActorLocation`) (`self.K2_GetActorRotation` _returnvalue))
  (`self.K2_DestroyActor`))

(fn `UserConstructionScript`)