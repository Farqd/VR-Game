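; Dart spawner actor that creates BP_dart instances, with an optional limited supply.
; BeginPlay calls TrySpawnDart, which spawns a dart at the DartSpawnPlace socket and passes itself as the dart's Spawner.
; When LimitedDarts is set, it spawns only while DartsLeft remains, decrementing the count and writing it to four text displays.
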(event `self.ReceiveBeginPlay`
  (`self.TrySpawnDart`))

(event `self.ReceiveTick`
  (params (DeltaSeconds :type "Float (single-precision)")))

(fn `CreateDart`
  (`|SpawnActorFromClass` "/Game/Blueprints/BP_dart.BP_dart_C" (`KismetMathLibrary.MakeTransform` (`SceneComponent.GetSocketLocation` (`self.dart_spawner`) "DartSpawnPlace") (struct) (1.0 1.0 1.0)) "Undefined" "OverrideRootScale" null self))

(fn `TrySpawnDart`
  (if (`self.LimitedDarts`)
    (if (> (`self.DartsLeft`) 0)
      (`/Engine/EditorBlueprintResources/StandardMacros.DecrementInt` (`self.DartsLeft`)
        (:`  `
          (`self.CreateDart`)
          (`self.UpdateDisplays`))))
    (else
      (`self.CreateDart`))))

(fn `UpdateDisplays`
  (`|ExecutionSequence`
    (:`then_0`
      (`TextRenderComponent.K2_SetText` (`self.text1`) (`KismetTextLibrary.Conv_StringToText` (`KismetStringLibrary.Conv_IntToString` (`self.DartsLeft`)))))
    (:`then_1`
      (`TextRenderComponent.K2_SetText` (`self.text2`) (`KismetTextLibrary.Conv_StringToText` (`KismetStringLibrary.Conv_IntToString` (`self.DartsLeft`)))))
    (:`then_2`
      (`TextRenderComponent.K2_SetText` (`self.text3`) (`KismetTextLibrary.Conv_StringToText` (`KismetStringLibrary.Conv_IntToString` (`self.DartsLeft`)))))
    (:`then_3`
      (`TextRenderComponent.K2_SetText` (`self.text4`) (`KismetTextLibrary.Conv_StringToText` (`KismetStringLibrary.Conv_IntToString` (`self.DartsLeft`)))))))

(fn `UserConstructionScript`)