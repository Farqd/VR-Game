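; Player pawn with camera-relative movement, look controls and a telekinesis ability for grabbing and carrying physics objects.
; Pressing grab line-traces from the camera and attaches a hit simulating component to the PhysicsHandle; releasing drops it.
; While held, Tick drives the handle toward the HandleLocation component, which an input axis slides along its forward vector, with a minimum camera distance limiting inward movement.
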(event `InputAxis|Turn`
  (params (AxisValue :type "Float (single-precision)"))
  (`self.AddControllerYawInput` AxisValue))

(event `InputAxis|MoveForward`
  (params (AxisValue :type "Float (single-precision)"))
  (`self.AddMovementInput` (`SceneComponent.GetForwardVector` (`self.Camera`)) AxisValue))

(event `InputAxis|MoveRight`
  (params (AxisValue :type "Float (single-precision)"))
  (`self.AddMovementInput` (`SceneComponent.GetRightVector` (`self.Camera`)) AxisValue))

(event `InputAxis|LookSky`
  (params (AxisValue :type "Float (single-precision)"))
  (`self.AddControllerPitchInput` AxisValue))

(event `InputAction|TelekinesisGrab`
  (params (Key :type "Key Structure" :default "AnyKey"))
  (bind _camera (`self.Camera`))
  (bind _returnvalue (`SceneComponent.K2_GetComponentLocation` _camera))
  (:`Pressed`
    (if (not (`self.isGrabing`))
      (bind (_outhit _returnvalue_2) (`KismetSystemLibrary.LineTraceSingle` :`Start` _returnvalue :`End` (+ _returnvalue (* (`SceneComponent.GetForwardVector` _camera) 10000.0)) :`TraceChannel` "TraceTypeQuery1" :`DrawDebugType` "ForDuration"))
      (if _returnvalue_2
        (bind (_bblockinghit _binitialoverlap _time _location _impactpoint _normal _impactnormal _physmat _hitactor _hitcomponent) (`GameplayStatics.BreakHitResult` _outhit))
        (if (`SceneComponent.IsSimulatingPhysics` _hitcomponent "None")
          (bind _returnvalue_3 (`SceneComponent.K2_GetComponentLocation` _hitcomponent))
          (`PhysicsHandleComponent.GrabComponentAtLocation` (`self.PhysicsHandle`) _hitcomponent "None" _returnvalue_3)
          (`SceneComponent.K2_SetWorldLocation` (`self.handleLocation`) _returnvalue_3 false false)
          (set `self.isGrabing` true)))))
  (:`Released`
    (if (`self.isGrabing`)
      (`PhysicsHandleComponent.ReleaseComponent` (`self.PhysicsHandle`))
      (set `self.isGrabing` false))))

(event `self.ReceiveTick`
  (params (DeltaSeconds :type "Float (single-precision)"))
  (if (`self.isGrabing`)
    (`PhysicsHandleComponent.SetTargetLocation` (`self.PhysicsHandle`) (`SceneComponent.K2_GetComponentLocation` (`self.handleLocation`)))))

(event `InputAxis|TelekinesisMoveFurther`
  (params (AxisValue :type "Float (single-precision)"))
  (bind _handlelocation (`self.handleLocation`))
  (if (and (`self.isGrabing`) (or (> (`KismetMathLibrary.VSize` (- (`SceneComponent.K2_GetComponentLocation` (`self.Camera`)) (`SceneComponent.K2_GetComponentLocation` _handlelocation))) (`self.minDistance`)) (> (`self.GetInputAxisValue`) 0.0)))
    (`SceneComponent.K2_AddWorldOffset` _handlelocation (* (* (`SceneComponent.GetForwardVector` _handlelocation) AxisValue) 5.0) false false)))

(fn `UserConstructionScript`)