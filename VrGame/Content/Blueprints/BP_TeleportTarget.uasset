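; BP_TeleportTarget is a projectile that teleports the player pawn to where it hits, then destroys itself.
; On a Sphere hit it moves player 0 to its location, keeping rotation, and retries 100 units higher if that fails.
; The construction script drives the ProjectileMovement speeds and forward velocity from a Speed variable.
; Debug prints remain on spawn, bounce, stop and hit, alongside an unconnected older teleport branch.
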(event `self.ReceiveBeginPlay`
  (`KismetSystemLibrary.PrintString` "spawned"))

(event `self.ProjectileMovement.OnProjectileBounce`
  (params (ImpactResult :type "HitResult Structure (by ref)") (ImpactVelocity :type "Vector Structure (by ref)"))
  (`KismetSystemLibrary.PrintString` "Hello" :!label _label))

(event `self.ProjectileMovement.OnProjectileStop`
  (params (ImpactResult :type "HitResult Structure (by ref)"))
  (goto _label))

(event `self.Sphere.OnComponentHit`
  (params (HitComponent :type "PrimitiveComponent Object Reference") (OtherActor :type "Actor Object Reference") (OtherComp :type "PrimitiveComponent Object Reference") (NormalImpulse :type "Vector Structure") (Hit :type "HitResult Structure (by ref)"))
  (bind _returnvalue (`GameplayStatics.GetPlayerPawn` 0))
  (bind _returnvalue_2 (`self.K2_GetActorLocation`))
  (bind _returnvalue_3 (`GameplayStatics.GetPlayerPawn` 0))
  (`KismetSystemLibrary.PrintString` (`KismetStringLibrary.Conv_ObjectToString` OtherActor))
  (bind _returnvalue_4 (`self.K2_TeleportTo` _returnvalue _returnvalue_2 (`self.K2_GetActorRotation` _returnvalue)))
  (if (not _returnvalue_4)
    (`self.K2_TeleportTo` _returnvalue_3 (+ _returnvalue_2 (`KismetMathLibrary.MakeVector` 0.0 0.0 100.0)) (`self.K2_GetActorRotation` _returnvalue_3)))
  (`self.K2_DestroyActor`))

(fn `UserConstructionScript`
  (`|ExecutionSequence`
    (:`then_0`
      (set `ProjectileMovementComponent.InitialSpeed` (`self.Speed`) (`self.ProjectileMovement`)))
    (:`then_1`
      (set `ProjectileMovementComponent.MaxSpeed` (`self.Speed`) (`self.ProjectileMovement`)))
    (:`then_2`
      (set `MovementComponent.Velocity` (`KismetMathLibrary.MakeVector` (`self.Speed`)) (`self.ProjectileMovement`)))))