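; BP_Trigger is a trigger actor that signals when qualifying actors begin or end overlapping it.
; Overlap events filter the other actor by interface, with BPI_TriggerActivator named on the end check and no interface specified on the begin check.
; Passing actors fire the TriggerStart or TriggerEnd event dispatcher, leaving the response to bound listeners.
; Each successful check also prints the actor's class name for debugging.
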(event `self.ReceiveActorBeginOverlap`
  (params (OtherActor :type "Actor Object Reference"))
  (if (`KismetSystemLibrary.DoesImplementInterface` OtherActor)
    (`self.TriggerStart`)
    (`KismetSystemLibrary.PrintString` (`KismetSystemLibrary.GetClassDisplayName` (`GameplayStatics.GetObjectClass` OtherActor)))))

(event `self.ReceiveActorEndOverlap`
  (params (OtherActor :type "Actor Object Reference"))
  (if (`KismetSystemLibrary.DoesImplementInterface` OtherActor "/Game/Blueprints/BPI_TriggerActivator.BPI_TriggerActivator_C")
    (`self.TriggerEnd`)
    (`KismetSystemLibrary.PrintString` (`KismetSystemLibrary.GetClassDisplayName` (`GameplayStatics.GetObjectClass` OtherActor)))))

(fn `UserConstructionScript`)